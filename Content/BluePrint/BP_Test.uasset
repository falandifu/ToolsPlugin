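; BP_Test is a test Blueprint that lays out a grid of hierarchical instanced static meshes from row and column counts.
; Its construction script clears the instances, then adds one per grid cell, so the layout rebuilds whenever the script runs.
; CalculateArrayPosition sets each instance's X and Y from row and column spacing, random offset ranges and a random stream.
; The event graph holds only disabled placeholder events.
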(event EventBeginPlay)

(event Collision|EventActorBeginOverlap
  (params (OtherActor :type Actor%20Object%20Reference)))

(event EventTick
  (params (DeltaSeconds :type Float%20%28single-precision%29)))

(fn ConstructionScript
  (bind _hierarchicalinstancedstaticmesh (Variables|Default|GetHierarchicalInstancedStaticMesh))
  (Components|InstancedStaticMesh|ClearInstances _hierarchicalinstancedstaticmesh)
  (for _index (range 0 (- (* (Variables|Default|Get行) (Variables|Default|Get列)) 1))
    (Components|InstancedStaticMesh|AddInstance _hierarchicalinstancedstaticmesh (Math|Transform|MakeTransform (Math|Vector|MakeVector (.X (Class|QuickToolBPLibrary|CalculateArrayPosition (Variables|Default|Get行) (Variables|Default|Get列) _index (Variables|Default|Get行间距) (Variables|Default|Get列间距) (Variables|Default|GetRow%20Distance%20Random%20Min) (Variables|Default|GetRow%20Distance%20Random%20Max) (Variables|Default|GetCoumn%20Distance%20Random%20Min) (Variables|Default|GetCoumn%20Distance%20Random%20Max) (Variables|Default|GetPosition%20Stream))) (.Y (Class|QuickToolBPLibrary|CalculateArrayPosition (Variables|Default|Get行) (Variables|Default|Get列) _index (Variables|Default|Get行间距) (Variables|Default|Get列间距) (Variables|Default|GetRow%20Distance%20Random%20Min) (Variables|Default|GetRow%20Distance%20Random%20Max) (Variables|Default|GetCoumn%20Distance%20Random%20Min) (Variables|Default|GetCoumn%20Distance%20Random%20Max) (Variables|Default|GetPosition%20Stream))) 0.0) "0, 0, 0" "1.000000,1.000000,1.000000") false)))